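; Lobby game mode that registers joining players, spawns their pawns and launches the match by server travel.
; PostLogin pulls server info from the game instance, sets up each BP_PC_Lobby and spawns a default character at a random PlayerStart.
; It pushes map settings, player lists and available characters to all controllers, and derives CanWeStart from character choices.
; SwapCharacter respawns players as another class; the kick-list event is an empty stub.
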(event Custom|SwapCharacter
  (params (PlayerController :type Player%20Controller%20Object%20Reference) (CharacterClass :type Character%20Class%20Reference) (ChangedStatus :type Boolean))
  (bind _returnvalue (Pawn|GetControlledPawn PlayerController))
  (bind _spawnpoint (Variables|ServerSettings|GetSpawnPoint))
  ;[1 1 1] Swaps the current character
  (if (not ChangedStatus)
    (Utilities|IsValid _returnvalue
      (:Is%20Valid
        (Actor|DestroyActor _returnvalue)
        (bind _returnvalue_2 (Game|SpawnActorfromClass CharacterClass (Transformation|GetActorTransform (Utilities|Array|Get(acopy) _spawnpoint (Math|Random|RandomIntegerinRange 0 (- (Utilities|Array|Length _spawnpoint) 1)))) "Undefined" 0 0))
        (Pawn|Possess PlayerController _returnvalue_2)))))

(event Custom|EveryoneUpdate
  (bind _allplayercontroller (Variables|ServerSettings|GetAllPlayerController))
  ;[1 1 1] Updates All connected players info when called
  (bind _output_get (Variables|ServerSettings|SetCurrentPlayers (Utilities|Array|Length (Variables|ServerSettings|GetAllPlayerController))))
  (if (> _output_get 0)
    (Utilities|Array|Clear (Variables|ServerSettings|GetConnectedPlayers))
    (for _array_element _allplayercontroller
      (bind _asbp_pc_lobby (Utilities|Casting|CastToBP_PC_Lobby _array_element))
      (Utilities|Array|Add (Variables|ServerSettings|GetConnectedPlayers) (Variables|/Game/Blueprints/Lobby/BP_PC_Lobby.BP_PC_Lobby_C|GetPlayerSettings _asbp_pc_lobby))
      (Default|UpdateNumberOfPlayers _asbp_pc_lobby (Variables|ServerSettings|GetCurrentPlayers) (Variables|ServerSettings|GetMaxPlayers)))
    (for _array_element_2 _allplayercontroller
      (bind _asbp_pc_lobby_2 (Utilities|Casting|CastToBP_PC_Lobby _array_element_2))
      (Default|AddPlayerInfo _asbp_pc_lobby_2 (Variables|ServerSettings|GetConnectedPlayers))
      (Default|UpdateAvailableCharacters _asbp_pc_lobby_2 (Variables|ServerSettings|GetAvailableCharacters))
      (CallFunction|AddtoKickList))
    (bind _array_element_3 (Utilities|Array|ForEachLoopwithBreak (Variables|ServerSettings|GetConnectedPlayers))
      (:LoopBody
        (if (== (.PlayerCharacter (Utilities|Struct|BreakBP_Struc_Player _array_element_3)) "/Game/Blueprints/Characters/BP_C_BasePlayer.BP_C_BasePlayer_C")
          (Variables|ServerSettings|SetCanWeStart false)
          (CallFunction|CannotStarGame)
          (else
            (Variables|ServerSettings|SetCanWeStart true)))))))

(event Custom|LauchTheGame
  ;[1 1 1] Launch game with selected map
  (switch int (Variables|ServerSettings|GetGM_MapID)
    (:0
      (Development|ExecuteConsoleCommand "servertravel /Game/Maps/UW_Proto01" 0))
    (:1
      (Development|ExecuteConsoleCommand "servertravel /Game/Maps/Underwater" (Game|GetPlayerController 0)))))

(event Custom|RespawnPlayer
  (params (PlayerController :type Player%20Controller%20Object%20Reference))
  (bind _returnvalue (Pawn|GetControlledPawn PlayerController))
  (bind _spawnpoint (Variables|ServerSettings|GetSpawnPoint))
  ;[1 1 1] Spawn the player as default Character
  (Utilities|IsValid _returnvalue
    (:Is%20Valid
      (Actor|DestroyActor _returnvalue))
    (:Is%20Not%20Valid
      _))
  (bind _returnvalue_2 (Game|SpawnActorfromClass "/Game/Blueprints/Characters/BP_C_BasePlayer.BP_C_BasePlayer_C" (Transformation|GetActorTransform (Utilities|Array|Get(acopy) _spawnpoint (Math|Random|RandomIntegerinRange 0 (- (Utilities|Array|Length _spawnpoint) 1)))) "Undefined" 0 0))
  (Pawn|Possess PlayerController _returnvalue_2)
  (CallFunction|EveryoneUpdate))

(event Custom|AddToKickList)

(event Custom|CannotStarGame
  ;[1 1 1] Updates All connected players info when called
  (Utilities|Array|ForEachLoopwithBreak (Variables|ServerSettings|GetConnectedPlayers)) ; enters at Break
)

(event Custom|ServerUpdateGameSettings
  (params (MapImage :type Texture%202D%20Object%20Reference) (MapName :type Text) (MapTime :type Text) (MapID :type Integer))
  ;[1 1 1] Server has made some change and call to update
  (Variables|ServerSettings|SetGM_MapImage MapImage)
  (Variables|ServerSettings|SetGM_Mapname MapName)
  (Variables|ServerSettings|SetGM_MapTime MapTime)
  (Variables|ServerSettings|SetGM_MapID MapID)
  (for _array_element (Variables|ServerSettings|GetAllPlayerController)
    (bind _asbp_pc_lobby (Utilities|Casting|CastToBP_PC_Lobby _array_element))
    (Default|UpdateLobbySettings _asbp_pc_lobby (Variables|ServerSettings|GetGM_MapImage) (Variables|ServerSettings|GetGM_Mapname) (Variables|ServerSettings|GetGM_MapTime))))

(event EventPostLogin
  (params (NewPlayer :type Player%20Controller%20Object%20Reference))
  ;[1 1 1] Initail Setup
  (Networking|SwitchHasAuthority
    (:Authority
      (Utilities|Array|Add (Variables|ServerSettings|GetAllPlayerController) NewPlayer)
      (bind _outactors (Actor|GetAllActorsOfClass "/Script/Engine.PlayerStart"))
      (Variables|ServerSettings|SetSpawnPoint _outactors)
      (bind _asbp_main_gi (Utilities|Casting|CastToBP_MainGI (Game|GetGameInstance)))
      (Variables|ServerSettings|SetServerName (Variables|/Game/Blueprints/Global/BP_MainGI.BP_MainGI_C|GetServerName _asbp_main_gi))
      (Variables|ServerSettings|SetMaxPlayers (Variables|/Game/Blueprints/Global/BP_MainGI.BP_MainGI_C|GetMaxPlayers _asbp_main_gi))
      (bind _asbp_pc_lobby (Utilities|Casting|CastToBP_PC_Lobby NewPlayer))
      (Default|InitialSetup _asbp_pc_lobby)
      (Default|SetupLobbyMenu _asbp_pc_lobby (Variables|ServerSettings|GetServerName))
      (Default|UpdateLobbySettings _asbp_pc_lobby (Variables|ServerSettings|GetGM_MapImage) (Variables|ServerSettings|GetGM_Mapname) (Variables|ServerSettings|GetGM_MapTime))
      (CallFunction|RespawnPlayer NewPlayer))))

(fn ConstructionScript)