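; Lobby game mode that manages connected players, character selection and map settings before launching the multiplayer match.
; On login it registers the player controller, sets up its lobby menu and possesses a default character at a random PlayerStart.
; EveryoneUpdate pushes player info, available characters and kick-list updates to controllers, and flags readiness based on non-default character picks.
; Logout frees the player's character; launch shows loading screens, then server-travels to the map selected by ID.
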(event Custom|SwapCharacter
  (params (PlayerController :type Player%20Controller%20Object%20Reference) (CharacterClass :type Character%20Class%20Reference) (ChangedStatus :type Boolean))
  (bind _returnvalue (Pawn|GetControlledPawn PlayerController))
  (bind _spawnpoint (Variables|ServerSettings|GetSpawnPoint))
  ;[1 1 1] Swaps the current character
  (if (not ChangedStatus)
    (Utilities|IsValid _returnvalue
      (:Is%20Valid
        (Actor|DestroyActor _returnvalue))
      (:Is%20Not%20Valid
        _))
    (bind _returnvalue_2 (Game|SpawnActorfromClass CharacterClass (Transformation|GetActorTransform (Utilities|Array|Get(acopy) _spawnpoint (- (Utilities|Array|Length _spawnpoint) 1))) "AlwaysSpawn" 0 0))
    (Pawn|Possess PlayerController _returnvalue_2)))

(event Custom|EveryoneUpdate
  (bind _connectedplayers (Variables|ServerSettings|GetConnectedPlayers))
  ;[1 1 1] Updates All connected players info when called
  (bind _output_get (Variables|ServerSettings|SetCurrentPlayers (Utilities|Array|Length (Variables|ServerSettings|GetConnectedPlayers))))
  (if (> _output_get 0)
    (Utilities|Array|Clear (Variables|Default|GetConnectedPlayersInfo))
    (for _array_element _connectedplayers
      (bind _lobbypc (Class|BPIPCLobby|LobbyPcRef(Message) _array_element))
      (Utilities|Array|Add (Variables|Default|GetConnectedPlayersInfo) (Variables|/Game/UnderWater/Blueprints/Lobby/BP_PC_Lobby.BP_PC_Lobby_C|GetPlayerSettings _lobbypc))
      (Default|UpdateNumberOfPlayers _lobbypc (Variables|ServerSettings|GetCurrentPlayers) (Variables|ServerSettings|GetMaxPlayers)))
    (for _array_element_2 _connectedplayers
      (bind _lobbypc_2 (Class|BPIPCLobby|LobbyPcRef(Message) _array_element_2))
      (Default|AddPlayerInfo _lobbypc_2 (Variables|Default|GetConnectedPlayersInfo))
      (Default|UpdateAvailableCharacters _lobbypc_2 (Variables|ServerSettings|GetAvailableCharacters))
      (CallFunction|AddtoKickList))
    (bind _array_element_3 (Utilities|Array|ForEachLoopwithBreak (Variables|Default|GetConnectedPlayersInfo))
      (:LoopBody
        (if (== (Utilities|Struct|BreakS_PlayerInfo _array_element_3) "/Game/UnderWater/Blueprints/Characters/BP_C_BasePlayer.BP_C_BasePlayer_C")
          (Variables|ServerSettings|SetCanWeStart false)
          (CallFunction|CannotStarGame)
          (else
            (Variables|ServerSettings|SetCanWeStart true)))))))

(event Custom|LauchTheGame
  (bind _returnvalue (Game|GetPlayerController 0))
  ;[1 1 1] Launch game with selected map
  (switch int (Variables|ServerSettings|GetGM_MapID)
    (:0
      (Development|ExecuteConsoleCommand "servertravel /Game/Maps/UW_Proto01" _returnvalue))
    (:1
      (Development|ExecuteConsoleCommand "servertravel /Game/Maps/Underwater" _returnvalue))))

(event Custom|RespawnPlayer
  (params (PlayerController :type Player%20Controller%20Object%20Reference))
  (bind _returnvalue (Pawn|GetControlledPawn PlayerController))
  (bind _spawnpoint (Variables|ServerSettings|GetSpawnPoint))
  ;[1 1 1] Spawn the player as default Character
  (Utilities|IsValid _returnvalue
    (:Is%20Valid
      (Actor|DestroyActor _returnvalue))
    (:Is%20Not%20Valid
      _))
  (bind _returnvalue_2 (Game|SpawnActorfromClass "/Game/UnderWater/Blueprints/Characters/BP_C_BasePlayer.BP_C_BasePlayer_C" (Transformation|GetActorTransform (Utilities|Array|Get(acopy) _spawnpoint (Math|Random|RandomIntegerinRange 0 (- (Utilities|Array|Length _spawnpoint) 1)))) "Undefined" 0 0))
  (Pawn|Possess PlayerController _returnvalue_2)
  (CallFunction|EveryoneUpdate))

(event Custom|AddToKickList
  ;[1 1 1] Add players to the Kick List
  (bind _lobbypc (Class|BPIPCLobby|LobbyPcRef(Message) (Game|GetPlayerController 0)))
  (Default|AddPlayertoKickWindow _lobbypc))

(event Custom|CannotStarGame
  ;[1 1 1] Updates All connected players info when called
  (Utilities|Array|ForEachLoopwithBreak (Variables|Default|GetConnectedPlayersInfo)) ; enters at Break
)

(event Custom|ServerUpdateGameSettings
  (params (MapImage :type Texture%202D%20Object%20Reference) (MapName :type Text) (MapTime :type Text) (MapID :type Integer))
  ;[1 1 1] Server has made some change and call to update
  (Variables|ServerSettings|SetGM_MapImage MapImage)
  (Variables|ServerSettings|SetGM_Mapname MapName)
  (Variables|ServerSettings|SetGM_MapTime MapTime)
  (Variables|ServerSettings|SetGM_MapID MapID)
  (for _array_element (Variables|ServerSettings|GetConnectedPlayers)
    (bind _asbp_pc_lobby (Utilities|Casting|CastToBP_PC_Lobby _array_element))
    (Default|UpdateLobbySettings _asbp_pc_lobby (Variables|ServerSettings|GetGM_MapImage) (Variables|ServerSettings|GetGM_Mapname) (Variables|ServerSettings|GetGM_MapTime))))

(event Custom|StartLoadingScreen
  ;[1 1 1] Launch game with selected map
  (for _array_element (Variables|ServerSettings|GetConnectedPlayers)
    (bind _lobbypc (Class|BPIPCLobby|LobbyPcRef(Message) _array_element))
    (Default|ShowLoadingScreen _lobbypc))
  (CallFunction|LauchtheGame))

(event EventPostLogin
  (params (NewPlayer :type Player%20Controller%20Object%20Reference))
  ;[1 1 1] Initail Setup
  (bind _output_get (Variables|Default|SetConnectedPlayer NewPlayer))
  (Utilities|Array|AddUnique (Variables|ServerSettings|GetConnectedPlayers) _output_get)
  (bind _outactors (Actor|GetAllActorsOfClass "/Script/Engine.PlayerStart"))
  (Variables|ServerSettings|SetSpawnPoint _outactors)
  (bind _gameinstance (Class|BPIMainGI|GameInstanceRef(Message) (Game|GetGameInstance)))
  (Variables|ServerSettings|SetServerName (Variables|/Game/UnderWater/Blueprints/_Main/BP_MainGI.BP_MainGI_C|GetServerName _gameinstance))
  (Variables|ServerSettings|SetMaxPlayers (Variables|/Game/UnderWater/Blueprints/_Main/BP_MainGI.BP_MainGI_C|GetMaxPlayers _gameinstance))
  (bind _lobbypc (Class|BPIPCLobby|LobbyPcRef(Message) NewPlayer))
  (bind _output_get_2 (Variables|Default|SetLobbyPC _lobbypc))
  (Default|InitialSetup _output_get_2)
  (Default|SetupLobbyMenu _output_get_2 (Variables|ServerSettings|GetServerName))
  (Default|UpdateLobbySettings _lobbypc (Variables|ServerSettings|GetGM_MapImage) (Variables|ServerSettings|GetGM_Mapname) (Variables|ServerSettings|GetGM_MapTime))
  (CallFunction|EveryoneUpdate)
  (CallFunction|RespawnPlayer NewPlayer))

(event EventOnLogout
  (params (ExitingController :type Controller%20Object%20Reference))
  (bind _connectedplayers (Variables|ServerSettings|GetConnectedPlayers))
  ;[1 1 1] Comment
  (bind (_array_element _array_index) (Utilities|Array|ForEachLoopwithBreak _connectedplayers :!label _label)
    (:LoopBody
      (if (== _array_element ExitingController)
        (goto _label Break)))
    (:Completed
      (bind _lobbypc (Class|BPIPCLobby|LobbyPcRef(Message) (Utilities|Array|Get(acopy) _connectedplayers _array_index)))
      (Utilities|Array|SetArrayElem (Variables|ServerSettings|GetAvailableCharacters) (Variables|/Game/UnderWater/Blueprints/Lobby/BP_PC_Lobby.BP_PC_Lobby_C|GetSelectedCharacter _lobbypc) false)
      (Utilities|Array|RemoveIndex (Variables|ServerSettings|GetConnectedPlayers) _array_index)
      (Utilities|Array|RemoveIndex (Variables|Default|GetConnectedPlayersInfo) _array_index)
      (CallFunction|EveryoneUpdate))))

(fn ConstructionScript)

(fn LobbyGMref
  (return self))