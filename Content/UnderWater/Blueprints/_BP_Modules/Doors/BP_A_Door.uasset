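; BP_A_Door is a networked sliding door that players open and close.
; On the server, its Box overlap tells BP_C_BasePlayer, via InteractWithDoor, when it enters or leaves range.
; OpenCloseDoor multicasts a vertical MoveComponentTo on SlidingDoor, then flips DoorOpen after a short delay.
; The DoorOpen RepNotify also sets the door's position, but its open height is lower than the animated target.
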(event OnComponentBeginOverlap(Box)
  (params (OverlappedComponent :type Primitive%20Component%20Object%20Reference) (OtherActor :type Actor%20Object%20Reference) (OtherComp :type Primitive%20Component%20Object%20Reference) (OtherBodyIndex :type Integer) (bFromSweep :type Boolean) (SweepResult :type Hit%20Result%20Structure%20%28by%20ref%29))
  (bind (_asbp_c_base_player _bsuccess) (Utilities|Casting|CastToBP_C_BasePlayer OtherActor))
  (Networking|SwitchHasAuthority
    (:Authority
      (if _bsuccess
        (Default|InteractwithDoor _asbp_c_base_player self true)))))

(event OnComponentEndOverlap(Box)
  (params (OverlappedComponent :type Primitive%20Component%20Object%20Reference) (OtherActor :type Actor%20Object%20Reference) (OtherComp :type Primitive%20Component%20Object%20Reference) (OtherBodyIndex :type Integer))
  (bind (_asbp_c_base_player _bsuccess) (Utilities|Casting|CastToBP_C_BasePlayer OtherActor))
  (Networking|SwitchHasAuthority
    (:Authority
      (if _bsuccess
        (Default|InteractwithDoor _asbp_c_base_player self false)))))

(event Custom|OpenCloseDoor
  (bind _slidingdoor (Variables|Default|GetSlidingDoor))
  (bind _slidingdoor_2 (Variables|Default|GetSlidingDoor))
  (bind _relativerotation (Variables|/Script/Engine.SceneComponent|GetRelativeRotation _slidingdoor))
  (if (not (Variables|Default|GetDoorOpen))
    (CallFunction|MultiDoorMovement _slidingdoor_2 "0.000000, 0,350.000000" _relativerotation)
    (Utilities|FlowControl|Delay 0.2)
    (Variables|Default|SetDoorOpen true)
    (else
      (CallFunction|MultiDoorMovement _slidingdoor_2 "0, 0, 0" _relativerotation)
      (Utilities|FlowControl|Delay 0.2)
      (Variables|Default|SetDoorOpen false))))

(event Custom|Multi_DoorMovement
  (params (Component :type Scene%20Component%20Object%20Reference) (TargetRelativeLocation :type Vector) (TargetRelativeRotation :type Rotator))
  (Components|MoveComponentTo Component TargetRelativeLocation TargetRelativeRotation false false 0.2 false))

(fn ConstructionScript)

(fn OnRepDoorOpen
  (bind _slidingdoor (Variables|Default|GetSlidingDoor))
  (if (Variables|Default|GetDoorOpen)
    (Transformation|SetRelativeLocation _slidingdoor "0.000000, 0,128.000000" true false)
    (else
      (Transformation|SetRelativeLocation _slidingdoor "0, 0, 0" true false))))

(fn OnRepSlidingDistance)