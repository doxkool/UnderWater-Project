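; Gameplay game mode that tracks player controllers, spawns player characters and handles logout.
; SpawnPlayer spawns the selected character at a random PlayerStart and possesses it, or only destroys the controlled pawn if one already exists.
; Controllers are recorded on controller swap, and logout asks the game instance to destroy the session through interface messages.
; GameplayGMRef returns the game mode itself.
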(event Custom|SpawnPlayer
  (params (PlayerController :type Player%20Controller%20Object%20Reference) (SelectedCharacter :type Character%20Class%20Reference))
  (bind _returnvalue (Pawn|GetControlledPawn PlayerController))
  ;[1 1 1] Spawn the player at random spawn point
  (bind _outactors (Actor|GetAllActorsOfClass "/Script/Engine.PlayerStart"))
  (Variables|Default|SetSpawnPoints _outactors)
  (Utilities|IsValid _returnvalue
    (:Is%20Valid
      (Actor|DestroyActor _returnvalue))
    (:Is%20Not%20Valid
      (bind _returnvalue_2 (Game|SpawnActorfromClass SelectedCharacter (Transformation|GetActorTransform (Utilities|Array|Get(acopy) (Variables|Default|GetSpawnPoints) (Math|Random|RandomIntegerinRange 0 (- (Utilities|Array|Length (Variables|Default|GetSpawnPoints)) 1)))) "Undefined" 0 0))
      (Pawn|Possess PlayerController _returnvalue_2))))

(event EventOnSwapPlayerControllers
  (params (OldPC :type Player%20Controller%20Object%20Reference) (NewPC :type Player%20Controller%20Object%20Reference))
  (Utilities|Array|Add (Variables|Default|GetAllplayerControllers) NewPC))

(event EventOnLogout
  (params (ExitingController :type Controller%20Object%20Reference))
  ;[1 1 1] On log out
  (bind _gameplaypc (Class|BPIPCGameplay|GameplayPCRef(Message) ExitingController))
  (bind _gameinstance (Class|BPIMainGI|GameInstanceRef(Message) (Game|GetGameInstance)))
  (Default|DestroySessionCaller _gameinstance _gameplaypc))

(fn ConstructionScript)

(fn GameplayGMRef
  (return self))