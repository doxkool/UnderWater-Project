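; Gameplay player controller that hands the player's chosen character to the game mode for spawning.
; On BeginPlay the local controller clears all widgets, including the loading screen, and reads player settings from the game instance.
; After a short delay it passes them to the server, which calls SpawnPlayer on the game mode, then SetupUI, which is empty here.
; Game instance and game mode are reached through message calls, and GameplayPCRef returns the controller itself.
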(event Custom|PassCharacterInfoToServer
  (params (PlayerSettings :type S%20Player%20Info%20Structure) (Character :type Character%20Class%20Reference))
  ;[1 1 1] send the info to the server
  (Variables|Default|SetPlayerSettings PlayerSettings)
  (bind _gamplaygmref (Class|BPIGMGameplay|GameplayGMRef(Message) (Game|GetGameMode)))
  (Default|SpawnPlayer _gamplaygmref self Character)
  (Utilities|FlowControl|Delay 0.2)
  (CallFunction|SetupUI))

(event Custom|SetupUI)

(event EventBeginPlay
  ;[1 1 1] Unload the loading screen
  (if (Pawn|IsLocalController)
    (Viewport|RemoveAllWidgets)
    (bind _playerinfo (Class|BPIMainGI|GetPlayerInfo(Message) (Game|GetGameInstance)))
    (bind _output_get (Variables|Default|SetPlayerSettings _playerinfo))
    (Development|PrintString (Utilities|GetClassDisplayName (Utilities|Struct|BreakS_PlayerInfo _output_get)) true true "(R=1.000000,G=0.000000,B=0.811130,A=1.000000)")
    (Utilities|FlowControl|Delay 0.2)
    (CallFunction|PassCharacterInfotoServer (Variables|Default|GetPlayerSettings) (Utilities|Struct|BreakS_PlayerInfo _output_get))))

(fn ConstructionScript)

(fn GameplayPCRef
  (return self))