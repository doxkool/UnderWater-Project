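; Main menu player controller that pulls the local player's Steam identity when play begins.
; After a short delay it checks for the Steam subsystem, printing an error if absent, then fetches the player name and medium avatar.
; These fill a PlayerInfo struct passed to the GameInstance through message calls, even if the avatar fetch fails.
; It then retrieves the friends list and checks for online friends in the same game, without acting on them.
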(event EventBeginPlay
  (bind _returnvalue (Game|GetGameInstance))
  (Utilities|FlowControl|Delay 0.2)
  (if (Class|AdvancedSessionsLibrary|HasOnlineSubsystem "STEAM")
    (Development|PrintString "Steam Online SubSystem loaded" true true "(R=0.000000,G=0.043849,B=1.000000,A=1.000000)" 1e+01)
    (bind _output_get (Variables|Default|SetPlayerName (Utilities|Text|ToText(String) (Class|AdvancedSessionsLibrary|GetPlayerName self))))
    (Development|PrintString (Utilities|String|Append "Steam Player Name : " (Utilities|String|ToString(Text) _output_get)) true true "(R=0.000000,G=0.043849,B=1.000000,A=1.000000)" 1e+01)
    (bind _returnvalue_2 (Class|AdvancedSteamFriendsLibrary|GetSteamFriendAvatar (Class|AdvancedSessionsLibrary|GetUniqueNetID self) "SteamAvatar_Medium")
      (:OnSuccess
        _)
      (:OnFailure
        _))
    (bind _structout (Utilities|Struct|SetmembersinS_PlayerInfo (Variables|Default|GetPlayerInfo) (Variables|Default|GetPlayerName) _returnvalue_2))
    (Class|BPIMainGI|SavePlayerInfo(Message) _returnvalue _structout)
    (Class|BPIMainGI|MainMenuPlayerInfo(Message) _returnvalue)
    (bind _results (|GetandStoreFriendsList self)
      (:OnSuccess
        (for _array_element _results
          (if (Utilities|Enum|Equal(Enum) (.OnlineState (Utilities|Struct|BreakBPFriendInfo _array_element)) "Online")
            (if (.bIsPlayingSameGame (Utilities|Struct|BreakBPFriendInfo _array_element))
              _)))))
    (else
      (Development|PrintString "Failed to load Steam Online SubSystem. Make sure Steam is running!" true true "(R=1.000000,G=0.000000,B=0.151855,A=1.000000)" 1e+01))))

(fn ConstructionScript)